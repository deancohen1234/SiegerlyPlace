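; Grenade actor that detonates automatically on a short fixed fuse after it spawns.
; BeginPlay waits out the delay, then calls Explode.
; Explode spawns an explosion particle effect and applies full, non-falloff radial damage credited to the instigator.
; It also draws a debug sphere at the blast point, then destroys the actor.
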(event Custom|Explode
  (bind _returnvalue (Transformation|GetActorLocation))
  (Effects|SpawnEmitteratLocation "/Game/StarterContent/Particles/P_Explosion.P_Explosion" _returnvalue)
  (Game|Damage|ApplyRadialDamage 0.0 _returnvalue (Variables|Default|GetDamageRadius) 0 0 self (Game|GetInstigatorController) true "ECC_Visibility")
  (Rendering|Debug|DrawDebugSphere _returnvalue 1e+02 12 "(R=0.000000,G=0.742964,B=1.000000,A=1.000000)" 1.0 1.0)
  (Actor|DestroyActor))

(event EventBeginPlay
  (Utilities|FlowControl|Delay 1.0)
  (CallFunction|Explode))

(fn ConstructionScript)