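; Lobby game mode that moves the session to the Crypt map once enough players have joined.
; On each PostLogin it counts the PlayerController actors and prints the total.
; At three or more it prints a notice and calls TravelToCrypt, which runs a ServerTravel console command to CryptMap through player controller 0.
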(event Custom|TravelToCrypt
  (Development|ExecuteConsoleCommand "ServerTravel CryptMap" (Game|GetPlayerController 0)))

(event EventPostLogin
  (params (NewPlayer :type Player%20Controller%20Object%20Reference))
  (bind _outactors (Actor|GetAllActorsOfClass "/Script/Engine.PlayerController"))
  (Development|PrintString (Utilities|String|ToString(Integer) (Utilities|Array|Length _outactors)) true true "(R=0.000000,G=0.660000,B=1.000000,A=1.000000)" 1e+01)
  (if (>= (Utilities|Array|Length _outactors) 3)
    (Development|PrintString "Travelling to Crypt" true true "(R=0.000000,G=0.660000,B=1.000000,A=1.000000)" 5.0)
    (CallFunction|TraveltoCrypt)))

(fn ConstructionScript)